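; Loading helper actor that shows a loading screen while streaming in levels and restoring the player's saved position.
; On BeginPlay it adds WBP_Loading, then after a short delay loops over LevelsToLoad, issuing non-blocking stream loads and removing entries.
; When the list empties, it moves the player pawn to the position in the "Default" save slot.
; It then removes the widget and notifies the main game mode that loading finished.
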(event `self.ReceiveBeginPlay`
  (set `self.MaimGameMode` (`/Game/Cours3/Core/BPFL_MainGame.GetMainGameMode`))
  (`|ExecutionSequence`
    (:`then_0`
      (bind _returnvalue (`|CreateWidget` "/Game/Cours3/UI/WBP_Loading.WBP_Loading_C" (`GameplayStatics.GetPlayerController` 0)))
      (`UserWidget.AddToViewport` _returnvalue 0)
      (set `self.LoadingScreen` _returnvalue))
    (:`then_1`
      (`KismetSystemLibrary.Delay` 0.1)
      (for (_array_element _array_index) (`self.LevelsToLoad`)
        (`GameplayStatics.LoadStreamLevelBySoftObjectPtr` _array_element true)
        (`KismetArrayLibrary.Array_Remove` (`self.LevelsToLoad`) _array_index)
        (if (< (`KismetArrayLibrary.Array_Length` (`self.LevelsToLoad`)) 1)
          (`|ExecutionSequence`
            (:`then_0`
              (bind _returnvalue_2 (`GameplayStatics.LoadGameFromSlot` "Default"))
              (bind _asbp_main_save_game (cast `/Game/Cours3/Core/SaveLoadSystem/BP_MainSaveGame` _returnvalue_2))
              (`self.K2_SetActorLocation` (`GameplayStatics.GetPlayerPawn` 0) (`/Game/Cours3/Core/SaveLoadSystem/BP_MainSaveGame.PlayerPosition` _asbp_main_save_game) false false))
            (:`then_1`
              (`Widget.RemoveFromParent` (`self.LoadingScreen`))
              (`/Game/Cours3/Core/BP_Main_GM.OnFinishedLoading` (`self.MaimGameMode`)))))))))

(fn `UserConstructionScript`)